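; Screen stimulus actor for a user study, showing info, count and clock panels and sending timestamps through an LSL outlet on overlap begin and end.
; Overlap, VR grab or trigger input, or a debug key starts the study with a ding and a Timeline that drives the clock, refreshed on Tick.
; With Mode set, it shows a public-speaking banner and schedules a first stage that updates the count.
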(event Custom|Begin%20Study
  (Development|PrintString "Begin Study" true true "(R=0.189238,G=1.000000,B=0.420069,A=1.000000)")
  (if (Variables|Default|GetMode)
    (Rendering|Components|TextRender|SetText (Variables|Default|GetInfoPanel) (Variables|Default|GetPublicSpeakingBanner))
    (Rendering|Components|TextRender|SetText (Variables|Default|GetCountPanel) (Variables|Default|GetCount))
    (bind _returnvalue (Utilities|Time|SetTimerbyEvent (delegate Custom|PS%20Stage%201) (Variables|Default|GetGap1)))
    (Rendering|Components|TextRender|SetText (Variables|Default|GetTimerPanel) (Utilities|Text|ToText(Float) (Class|KismetSystemLibrary|GetTimerElapsedTimeHandle _returnvalue) "HalfToEven"))))

(event Custom|PS%20Stage%201
  (Development|PrintString "PS Stage 1")
  (bind _output_get (Variables|Default|SetCount "02"))
  (Rendering|Components|TextRender|SetText (Variables|Default|GetCountPanel) _output_get)
  (Utilities|Time|SetTimerbyEvent 0 0.0))

(event Custom|ResetTimer
  (bind _time_output (Timeline|Timer PlayFromStart)
    (:Update
      (Variables|Default|SetSeconds (Math|Float|Truncate _time_output)))
    (:Finished
      (Variables|Default|SetMinutes (+ (Variables|Default|GetMinutes) 1.0))
      (if (>= (Variables|Default|GetMinutes) 6e+01)
        (Variables|Default|SetHours (+ (Variables|Default|GetHours) 1.0))
        (Variables|Default|SetMinutes 0)
        (CallFunction|ResetTimer)))))

(event Input|EnhancedActionEvents|EnhancedInputActionLeftTriggerPull
  (params (ActionValue :type Boolean) (ElapsedSeconds :type Float%20%28double-precision%29) (TriggeredSeconds :type Float%20%28double-precision%29) (InputAction :type Input%20Action%20Object%20Reference :default "/Game/BluePrints/LeftTriggerPull.LeftTriggerPull"))
  (CallFunction|BeginStudy)
  (Audio|PlaySound2D "/Game/long_ding.long_ding" 1.0 1.0 0.0 0 0)
  (bind _time_output (Timeline|Timer Play)
    (:Update
      (Variables|Default|SetSeconds (Math|Float|Truncate _time_output)))
    (:Finished
      (Variables|Default|SetMinutes (+ (Variables|Default|GetMinutes) 1.0))
      (if (>= (Variables|Default|GetMinutes) 6e+01)
        (Variables|Default|SetHours (+ (Variables|Default|GetHours) 1.0))
        (Variables|Default|SetMinutes 0)
        (CallFunction|ResetTimer)))))

(event Input|EnhancedActionEvents|EnhancedInputActionIA_Grab_Left
  (params (ActionValue :type Float%20%28double-precision%29) (ElapsedSeconds :type Float%20%28double-precision%29) (TriggeredSeconds :type Float%20%28double-precision%29) (InputAction :type Input%20Action%20Object%20Reference :default "/Game/VRTemplate/Input/Actions/IA_Grab_Left.IA_Grab_Left"))
  (CallFunction|BeginStudy)
  (Audio|PlaySound2D "/Game/long_ding.long_ding" 1.0 1.0 0.0 0 0)
  (bind _time_output (Timeline|Timer Play)
    (:Update
      (Variables|Default|SetSeconds (Math|Float|Truncate _time_output)))
    (:Finished
      (Variables|Default|SetMinutes (+ (Variables|Default|GetMinutes) 1.0))
      (if (>= (Variables|Default|GetMinutes) 6e+01)
        (Variables|Default|SetHours (+ (Variables|Default|GetHours) 1.0))
        (Variables|Default|SetMinutes 0)
        (CallFunction|ResetTimer)))))

(event EventBeginPlay
  (Input|EnableInput (Game|GetPlayerController 0)))

(event Collision|EventActorBeginOverlap
  (params (OtherActor :type Actor%20Object%20Reference))
  (Class|LSLOutletComponent|PushSampleString (Variables|Default|GetLSLOutlet) (Utilities|Array|MakeArray (Variables|Default|GetTime)))
  (CallFunction|BeginStudy)
  (Audio|PlaySound2D "/Game/long_ding.long_ding" 1.0 1.0 0.0 0 0)
  (bind _time_output (Timeline|Timer Play)
    (:Update
      (Variables|Default|SetSeconds (Math|Float|Truncate _time_output)))
    (:Finished
      (Variables|Default|SetMinutes (+ (Variables|Default|GetMinutes) 1.0))
      (if (>= (Variables|Default|GetMinutes) 6e+01)
        (Variables|Default|SetHours (+ (Variables|Default|GetHours) 1.0))
        (Variables|Default|SetMinutes 0)
        (CallFunction|ResetTimer)))))

(event EventTick
  (params (DeltaSeconds :type Float%20%28single-precision%29))
  (bind _output_get (Variables|Default|SetTime (Utilities|String|Append (Utilities|String|Right (Utilities|String|Append "0" (Utilities|String|ToString(Integer) (Variables|Default|GetHours))) 2) ":" (Utilities|String|Right (Utilities|String|Append "0" (Utilities|String|ToString(Integer) (Variables|Default|GetMinutes))) 2) ":" (Utilities|String|Right (Utilities|String|Append "0" (Utilities|String|ToString(Integer) (Variables|Default|GetSeconds))) 2))))
  (Rendering|Components|TextRender|SetText (Variables|Default|GetTimerPanel) (Utilities|Text|ToText(String) _output_get)))

(event Collision|EventActorEndOverlap
  (params (OtherActor :type Actor%20Object%20Reference))
  (Class|LSLOutletComponent|PushSampleString (Variables|Default|GetLSLOutlet) (Utilities|Array|MakeArray (Variables|Default|GetTime))))

(event Input|KeyboardEvents|DebugKeyS
  (params (Key :type Key%20Structure :default "None") (ActionValue :type Input%20Action%20Value%20Structure))
  (:Pressed
    (CallFunction|BeginStudy)
    (Audio|PlaySound2D "/Game/long_ding.long_ding" 1.0 1.0 0.0 0 0)
    (bind _time_output (Timeline|Timer Play)
      (:Update
        (Variables|Default|SetSeconds (Math|Float|Truncate _time_output)))
      (:Finished
        (Variables|Default|SetMinutes (+ (Variables|Default|GetMinutes) 1.0))
        (if (>= (Variables|Default|GetMinutes) 6e+01)
          (Variables|Default|SetHours (+ (Variables|Default|GetHours) 1.0))
          (Variables|Default|SetMinutes 0)
          (CallFunction|ResetTimer))))))

(fn ConstructionScript)